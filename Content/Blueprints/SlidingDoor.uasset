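; SlidingDoor is a door that opens once when the player presses F with a "Swipe Card" in their inventory.
; Overlap with a ThirdPersonCharacter toggles input on the actor, and F also checks that the player is inside the Collision component.
; Despite the name, a timeline swings the door by yaw, combined with the actor's rotation and applied as relative rotation, then marks it unlocked on finish.
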(event `self.ReceiveActorEndOverlap`
  (params (OtherActor :type "Actor Object Reference"))
  (cast `/Game/ThirdPersonCPP/Blueprints/ThirdPersonCharacter` OtherActor)
  (`self.DisableInput` (`GameplayStatics.GetPlayerController` 0)))

(event `self.ReceiveBeginPlay`
  (set `self.IsUnlocked` false))

(event `self.ReceiveActorBeginOverlap`
  (params (OtherActor :type "Actor Object Reference"))
  (cast `/Game/ThirdPersonCPP/Blueprints/ThirdPersonCharacter` OtherActor)
  (`self.EnableInput` (`GameplayStatics.GetPlayerController` 0)))

(event `Key|F`
  (params (Key :type "Key Structure"))
  (:`Pressed`
    (set `self.Rotation` (`self.K2_GetActorRotation`))
    (if (and (`PrimitiveComponent.IsOverlappingActor` (`self.Collision`) (`GameplayStatics.GetPlayerCharacter` 0)) (`BlueprintMapLibrary.Map_Find` (`/Game/ThirdPersonCPP/Blueprints/ThirdPersonCharacter.Inventory` (cast `/Game/ThirdPersonCPP/Blueprints/ThirdPersonCharacter` (`GameplayStatics.GetPlayerCharacter` 0) :!pure true)) "Swipe Card") (not (`self.IsUnlocked`)))
      (bind (_direction _door_rot) (`Timeline|Timeline_0`)
        (:`Update`
          (`SceneComponent.K2_SetRelativeRotation` (`self.Door`) (`KismetMathLibrary.ComposeRotators` (`KismetMathLibrary.MakeRotator` 0.0 0.0 _door_rot) (`self.Rotation`)) false false))
        (:`Finished`
          (set `self.IsUnlocked` true))))))

(fn `UserConstructionScript`)