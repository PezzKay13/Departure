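; Key pickup actor that lets the player collect a gold key by pressing F while something overlaps it.
; Begin and end overlap toggle a flag; on F, the last overlapping actor is cast to ThirdPersonCharacter, GoldKey is added to its Inventory, and the pickup destroys itself.
; Input is enabled for the first player controller on BeginPlay, and Tick turns an Arrow component to face the player camera.
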(event `self.ReceiveActorBeginOverlap`
  (params (OtherActor :type "Actor Object Reference"))
  (set `self.IsOverlapped` true))

(event `Key|F`
  (params (Key :type "Key Structure"))
  (:`Pressed`
    (if (`self.IsOverlapped`)
      (bind _asthird_person_character (cast `/Game/ThirdPersonCPP/Blueprints/ThirdPersonCharacter` (stale `self.ReceiveActorBeginOverlap` OtherActor)))
      (`BlueprintMapLibrary.Map_Add` (`/Game/ThirdPersonCPP/Blueprints/ThirdPersonCharacter.Inventory` _asthird_person_character) (`self.GoldKey`) true)
      (`self.K2_DestroyActor`))))

(event `self.ReceiveActorEndOverlap`
  (params (OtherActor :type "Actor Object Reference"))
  (set `self.IsOverlapped` false))

(event `self.ReceiveBeginPlay`
  (`self.EnableInput` (`GameplayStatics.GetPlayerController` 0)))

(event `self.ReceiveTick`
  (params (DeltaSeconds :type "Float (single-precision)"))
  (`SceneComponent.K2_SetWorldRotation` (`self.Arrow`) (`KismetMathLibrary.FindLookAtRotation` (`SceneComponent.K2_GetComponentLocation` (`self.Arrow`)) (`SceneComponent.K2_GetComponentLocation` (`PlayerCameraManager.TransformComponent` (`GameplayStatics.GetPlayerCameraManager` 0)))) false false))

(fn `UserConstructionScript`
  (`parent.UserConstructionScript`))