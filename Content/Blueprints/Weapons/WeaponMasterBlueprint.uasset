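; Master weapon Blueprint that provides a skeleton for networked start and stop firing.
; StartFire and StopFire forward remote calls to the server through ServerStartFire and ServerStopFire events.
; StartFire calls an empty CameraAim and prints a placeholder "Pew" while WantsToFire is false.
; The flag looks inverted: StartFire sets it false and StopFire sets it true, which blocks later firing.
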(event `ServerStartFire`
  (`self.StartFire`))

(event `ServerStopFire`
  (`self.StopFire`))

(fn `CameraAim`)

(fn `StartFire`
  (`/Engine/EditorBlueprintResources/ActorMacros.Switch Has Authority`
    (:`Authority`
      _)
    (:`Remote`
      (`self.ServerStartFire`)))
  (if (not (`self.WantsToFire`))
    (set `self.WantsToFire` false)
    (`self.CameraAim`)
    (`KismetSystemLibrary.PrintString` "Pew" true true (struct :`R` 1.0 :`B` 0.007941 :`A` 1.0))))

(fn `StopFire`
  (`/Engine/EditorBlueprintResources/ActorMacros.Switch Has Authority`
    (:`Authority`
      _)
    (:`Remote`
      (`self.ServerStopFire`)))
  (if (not (`self.WantsToFire`))
    (set `self.WantsToFire` true)))

(fn `UserConstructionScript`)