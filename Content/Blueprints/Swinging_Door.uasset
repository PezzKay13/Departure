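; Swinging double door that the player opens with F while overlapping it, requiring both a Gold Key and a Silver Key.
; Overlap toggles input, and pressing F checks the ThirdPersonCharacter's Inventory map, revealing the door's matching key mesh for each key held.
; With both keys, the DoorRotate timeline adds yaw to each leaf's captured world rotation, then marks the door open so it stays that way.
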(event `self.ReceiveBeginPlay`
  (`SceneComponent.SetVisibility` (`self.GoldKey`) false false)
  (`SceneComponent.SetVisibility` (`self.SilverKey`) false false)
  (set `self.Silver` false)
  (set `self.Gold` false)
  (set `self.Overlapping` false)
  (set `self.Open` false))

(event `self.ReceiveActorBeginOverlap`
  (params (OtherActor :type "Actor Object Reference"))
  (set `self.Overlapping` true)
  (`self.EnableInput` (`GameplayStatics.GetPlayerController` 0)))

(event `self.ReceiveActorEndOverlap`
  (params (OtherActor :type "Actor Object Reference"))
  (set `self.Overlapping` false)
  (`self.DisableInput` (`GameplayStatics.GetPlayerController` 0)))

(event `Key|F`
  (params (Key :type "Key Structure"))
  (:`Pressed`
    (set `self.LeftDoorRot` (`SceneComponent.K2_GetComponentRotation` (`self.DoorLeft`)))
    (set `self.RightDoorRot` (`SceneComponent.K2_GetComponentRotation` (`self.DoorRight`)))
    (if (`BlueprintMapLibrary.Map_Find` (`/Game/ThirdPersonCPP/Blueprints/ThirdPersonCharacter.Inventory` (cast `/Game/ThirdPersonCPP/Blueprints/ThirdPersonCharacter` (`GameplayStatics.GetPlayerCharacter` 0) :!pure true)) "Gold Key")
      (set `self.Gold` true)
      (`SceneComponent.SetVisibility` (`self.GoldKey`) true false))
    (if (`BlueprintMapLibrary.Map_Find` (`/Game/ThirdPersonCPP/Blueprints/ThirdPersonCharacter.Inventory` (cast `/Game/ThirdPersonCPP/Blueprints/ThirdPersonCharacter` (`GameplayStatics.GetPlayerCharacter` 0) :!pure true)) "Silver Key")
      (set `self.Silver` true)
      (`SceneComponent.SetVisibility` (`self.SilverKey`) true false))
    (if (and (`self.Gold`) (`self.Silver`) (not (`self.Open`)))
      (bind (_direction _rightdoor _leftdoor) (`Timeline|Door Rotate`)
        (:`Update`
          (`SceneComponent.K2_SetWorldRotation` (`self.DoorRight`) (`KismetMathLibrary.ComposeRotators` (`KismetMathLibrary.MakeRotator` 0.0 0.0 _rightdoor) (`self.RightDoorRot`)) false false)
          (`SceneComponent.K2_SetWorldRotation` (`self.DoorLeft`) (`KismetMathLibrary.ComposeRotators` (`KismetMathLibrary.MakeRotator` 0.0 0.0 _leftdoor) (`self.LeftDoorRot`)) false false))
        (:`Finished`
          (set `self.Open` true))))))

(fn `UserConstructionScript`)