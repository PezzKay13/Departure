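; Fire hazard actor that damages a DepartureCharacter and blocks its healing while it stands inside the Trigger volume.
; Begin and end overlap toggle the IsOnFire flag and the character's CanHeal flag.
; Tick applies a fixed, per-frame health loss while the flag is set, but targets the character reference from the end-overlap cast, not the begin-overlap one.
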(event `self.Trigger.OnComponentBeginOverlap`
  (params (OverlappedComponent :type "PrimitiveComponent Object Reference") (OtherActor :type "Actor Object Reference") (OtherComp :type "PrimitiveComponent Object Reference") (OtherBodyIndex :type Integer) (bFromSweep :type Boolean) (SweepResult :type "HitResult Structure (by ref)"))
  (bind _asdeparture_character (cast `DepartureCharacter` OtherActor))
  (set `self.IsOnFire` true)
  (set `DepartureCharacter.CanHeal` false _asdeparture_character))

(event `self.Trigger.OnComponentEndOverlap`
  (params (OverlappedComponent :type "PrimitiveComponent Object Reference") (OtherActor :type "Actor Object Reference") (OtherComp :type "PrimitiveComponent Object Reference") (OtherBodyIndex :type Integer))
  (bind _asdeparture_character (cast `DepartureCharacter` OtherActor))
  (set `self.IsOnFire` false)
  (set `DepartureCharacter.CanHeal` true _asdeparture_character))

(event `self.ReceiveTick`
  (params (DeltaSeconds :type "Float (single-precision)"))
  (if (`self.IsOnFire`)
    (`DepartureCharacter.UpdateHealth` (stale `self.Trigger.OnComponentEndOverlap` _asdeparture_character) -0.25)))

(fn `UserConstructionScript`)